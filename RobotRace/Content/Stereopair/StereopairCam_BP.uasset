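; Stereopair camera Blueprint that exports a depth and a raw render of its view when the 0 key is pressed.
; BeginPlay builds post-process settings and assigns render targets to two SceneCapture2D components, but the node applying those settings, including the depth material, is disconnected.
; The key press captures both components and exports the targets under CameraName with _d and _r suffixes.
; OutRenderFilePath's path-building nodes are unused.
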(event EventBeginPlay
  (Input|EnableInput (Game|GetPlayerController 0))
  (bind (_depthppsettings _rawppsettings) (CallFunction|ConstructPostProcessMaterialBlendables))
  (bind _output_get (Variables|Default|SetDepthPPSettings _depthppsettings))
  (bind _output_get_2 (Variables|Default|SetRawPPSettings _rawppsettings))
  (CallFunction|SetupSceneCaptureComponent _output_get (Variables|Default|GetDepthRenderTarget) (Variables|Default|GetDepthSceneCaptureComponent2D))
  (CallFunction|SetupSceneCaptureComponent _output_get_2 (Variables|Default|GetRawRenderTarget) (Variables|Default|GetRawSceneCaptureComponent2D)))

(event Collision|EventActorBeginOverlap
  (params (OtherActor :type Actor%20Object%20Reference)))

(event EventTick
  (params (DeltaSeconds :type Float%20%28single-precision%29)))

(event Input|KeyboardEvents|0
  (params (Key :type Key%20Structure :default "None"))
  (:Pressed
    (CallFunction|ExportCurrentFrametoFiles)
    (Development|PrintString (Utilities|String|Append (Variables|Default|GetCameraName) ": exported"))))

(fn ConstructionScript)

(fn ExportCurrentFrametoFiles
  (bind _cameraname (Variables|Default|GetCameraName))
  (bind _cameraname_2 (Variables|Default|GetCameraName))
  (bind _returnvalue (Utilities|String|Append _cameraname "_r"))
  (bind _returnvalue_2 (Utilities|String|Append _cameraname_2 "_d"))
  (bind (_path _filename) (Utilities|OutRenderFilePath _returnvalue))
  (bind (_path_2 _filename_2) (Utilities|OutRenderFilePath _returnvalue_2))
  (Rendering|SceneCapture|CaptureScene (Variables|Default|GetDepthSceneCaptureComponent2D) :!class /Script/Engine.SceneCaptureComponent2D)
  (Rendering|SceneCapture|CaptureScene (Variables|Default|GetRawSceneCaptureComponent2D) :!class /Script/Engine.SceneCaptureComponent2D)
  (Rendering|ExportRenderTarget (Variables|Default|GetDepthRenderTarget) _path_2 _filename_2)
  (Rendering|ExportRenderTarget (Variables|Default|GetRawRenderTarget) _path _filename))

(fn ConstructPostProcessMaterialBlendables
  (return (Utilities|Struct|MakePostProcessSettings (Utilities|Struct|MakeWeightedBlendables (Utilities|Array|MakeArray (Utilities|Struct|MakeWeightedBlendable 1.0 (Variables|Default|GetDepthPostProcessMaterial))))) (Utilities|Struct|MakePostProcessSettings (Utilities|Struct|MakeWeightedBlendables (Utilities|Array|MakeArray "")))))

(fn SetupSceneCaptureComponent
  (params (PostProcessingSettings :type Post%20Process%20Settings%20Structure) (RenderTarget :type Texture%20Render%20Target%202D%20Object%20Reference) (Target :type Scene%20Capture%20Component%202D%20Object%20Reference))
  (Variables|/Script/Engine.SceneCaptureComponent2D|SetTextureTarget Target RenderTarget))